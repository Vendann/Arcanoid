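; Player controller for the Arcanoid game that drives the paddle pawn, manages the HUD and resolves win or lose.
; Horizontal input moves the possessed pawn along Y with sweep, while actions spawn a ball or return to the main menu.
; The cube generator's cubes-destroyed event triggers a win and the pawn's game-over event a loss.
; Both play a sound, then share one path that swaps the HUD for WBP_WinScreen in UI-only input.
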(event Custom|GameOver
  (Audio|PlaySoundatLocation "/Game/Arcanoid/Sounds/Win_Cue.Win_Cue" "0, 0, 0" "0, 0, 0" 1.0 1.0 0.0 0 0 0 0)
  (Variables|Default|SetisWinner true)
  (Widget|SetVisibility (Variables|Default|GetHUD) "Collapsed")
  (bind _returnvalue (UserInterface|CreateWidget "/Game/Arcanoid/UI/WBP_WinScreen.WBP_WinScreen_C" self))
  (Default|GameOverText _returnvalue (Variables|Default|GetisWinner))
  (UserInterface|Viewport|AddtoViewport _returnvalue 0)
  (Input|SetInputModeUIOnly self _returnvalue "LockOnCapture" false)
  (Variables|Default|SetbShowMouseCursor true))

(event Custom|GameOver2
  (Audio|PlaySoundatLocation "/Game/Arcanoid/Sounds/Lose_Cue.Lose_Cue" "0, 0, 0" "0, 0, 0" 1.0 1.0 0.0 0 0 0 0)
  (Variables|Default|SetisWinner false)
  (Widget|SetVisibility (Variables|Default|GetHUD) "Collapsed")
  (bind _returnvalue (UserInterface|CreateWidget "/Game/Arcanoid/UI/WBP_WinScreen.WBP_WinScreen_C" self))
  (Default|GameOverText _returnvalue (Variables|Default|GetisWinner))
  (UserInterface|Viewport|AddtoViewport _returnvalue 0)
  (Input|SetInputModeUIOnly self _returnvalue "LockOnCapture" false)
  (Variables|Default|SetbShowMouseCursor true))

(event EventBeginPlay
  (Utilities|FlowControl|Sequence
    (:then_0
      (Input|SetInputModeGameOnly self false)
      (bind _returnvalue (UserInterface|CreateWidget "/Game/Arcanoid/UI/WBP_HUD.WBP_HUD_C" self))
      (UserInterface|Viewport|AddtoViewport _returnvalue 0)
      (Variables|Default|SetHUD _returnvalue))
    (:then_1
      (bind _returnvalue_2 (Actor|GetActorOfClass "/Game/Arcanoid/Blueprints/BP_CubeGenerator.BP_CubeGenerator_C"))
      (EventDispatchers|BindEventtoCubesDestroyed _returnvalue_2 (delegate Custom|GameOver)))))

(event EventPossess
  (params (PossessedPawn :type Pawn%20Object%20Reference))
  (bind _asbp_player_pawn (Utilities|Casting|CastToBP_PlayerPawn PossessedPawn))
  (bind _output_get (Variables|Default|SetPlayerPawn _asbp_player_pawn))
  (Variables|Default|SetisWinner false)
  (EventDispatchers|BindEventtoGameOver _output_get (delegate Custom|GameOver2)))

(event Input|ActionEvents|InputActionSpawnBall
  (params (Key :type Key%20Structure :default "None"))
  (:Pressed
    (Default|SpawnBall (Variables|Default|GetPlayerPawn))))

(event Input|ActionEvents|InputActionEscape
  (params (Key :type Key%20Structure :default "None"))
  (:Pressed
    (Game|OpenLevel(byObjectReference) "/Game/Arcanoid/Levels/L_MainMenu.L_MainMenu")))

(event Input|AxisEvents|InputAxisHorizontal
  (params (AxisValue :type Float%20%28single-precision%29))
  (bind _returnvalue (Math|Vector|Normalize (Math|Vector|MakeVector 0.0 AxisValue 0.0)))
  (Development|PrintString (Utilities|String|ToString(Float) (.y _returnvalue)))
  (Transformation|AddActorWorldOffset (Variables|Default|GetPlayerPawn) (Math|Vector|MakeVector 0.0 (* (.y _returnvalue) (Utilities|Time|GetWorldDeltaSeconds) (Variables|Default|GetSpeed)) 0.0) true))

(fn ConstructionScript)