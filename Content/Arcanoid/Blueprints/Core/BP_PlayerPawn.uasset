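; Player paddle pawn for an Arkanoid-style game that owns the ball spawn, lives and score.
; SpawnBall launches one main ball from the Arrow; its destruction costs a life, then shows the text prompt or signals game over.
; Cube overlaps consume bonuses for a timed paddle widen, extra life or smaller extra ball, plus sound and points.
; HP, score and game-over changes go out through event dispatchers.
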(event OnComponentBeginOverlap(Cube)
  (params (OverlappedComponent :type Primitive%20Component%20Object%20Reference) (OtherActor :type Actor%20Object%20Reference) (OtherComp :type Primitive%20Component%20Object%20Reference) (OtherBodyIndex :type Integer) (bFromSweep :type Boolean) (SweepResult :type Hit%20Result%20Structure%20%28by%20ref%29))
  ;[1 1 1] Overlap
  (bind _asbp_bonus (Utilities|Casting|CastToBP_Bonus OtherActor))
  (switch Utilities|FlowControl|Switch|SwitchonE_BonusType (Variables|/Game/Arcanoid/Blueprints/Bonuses/BP_Bonus.BP_Bonus_C|GetBonusType _asbp_bonus)
    (:NewEnumerator0
      (CallFunction|Max))
    (:NewEnumerator1
      (CallFunction|Live))
    (:NewEnumerator2
      (CallFunction|Ball)))
  (Audio|PlaySoundatLocation "/Game/Arcanoid/Sounds/Bonus_Cue.Bonus_Cue" (Transformation|GetActorLocation) "0, 0, 0" 1.0 1.0 0.0 0 0 0 0)
  (Actor|DestroyActor _asbp_bonus)
  (CallFunction|AddedScore 5))

(event Custom|SpawnBall
  ;[1 1 1] Spawner
  (if (not (<= (Variables|Default|GetPlayerHP) 0))
    (Variables|Default|GetSpawnedBall
      (:then)
      (:else
        (bind _returnvalue (Game|SpawnActorfromClass "/Game/Arcanoid/Blueprints/BP_Ball.BP_Ball_C" (Math|Transform|MakeTransform (Transformation|GetWorldLocation (Variables|Default|GetArrow))) "Undefined" "MultiplyWithRoot" 0 0))
        (bind _output_get (Variables|Default|SetSpawnedBall _returnvalue))
        (Game|BindEventtoOnDestroyed _output_get (delegate Custom|BallDead))
        (Rendering|SetVisibility (Variables|Default|GetTextRender) false false)))))

(event Custom|BallDead
  (params (DestroyedActor :type Actor%20Object%20Reference))
  ;[1 1 1] Spawner
  (bind _result (Math|Integer|DecrementInt (Variables|Default|GetPlayerHP))
    (:%20%20
      (Default|CallChangeHP _result)
      (if (<= _result 0)
        (Default|CallGameOver)
        (else
          (Rendering|SetVisibility (Variables|Default|GetTextRender) true false))))))

(event Custom|Ball
  ;[1 1 1] Spawn Smaller Ball
  (bind _returnvalue (Game|SpawnActorfromClass "/Game/Arcanoid/Blueprints/BP_Ball.BP_Ball_C" (Math|Transform|MakeTransform (Transformation|GetWorldLocation (Variables|Default|GetArrow)) "0, 0, 0" "0.500000,0.500000,0.500000") "Undefined" "MultiplyWithRoot" 0 0))
  (Default|DestroyingSmaller _returnvalue))

(event Custom|Max
  (bind _cube (Variables|Default|GetCube))
  (bind _relativescale3d (Variables|/Script/Engine.SceneComponent|GetRelativeScale3D _cube))
  ;[1 1 1] Increase Scale
  (if (not (Variables|Default|GetisScaled))
    (Transformation|SetRelativeScale3D _cube (Math|Vector|MakeVector (.x _relativescale3d) (* (.y _relativescale3d) 2.0) (.z _relativescale3d)))
    (CallFunction|ResetScale)
    (Variables|Default|SetisScaled true)))

(event Custom|Live
  ;[1 1 1] Increase Lives
  (bind _result (Math|Integer|IncrementInt (Variables|Default|GetPlayerHP))
    (:%20%20
      (Default|CallChangeHP _result))))

(event Custom|ResetScale
  ;[1 1 1] Reset Scale
  (Utilities|FlowControl|RetriggerableDelay 5.0)
  (Transformation|SetRelativeScale3D (Variables|Default|GetCube) (Variables|Default|GetRelative%20Scale%203D))
  (Variables|Default|SetisScaled false))

(event EventBeginPlay
  ;[1 1 1] Begin Play
  (Variables|Default|SetRelative%20Scale%203D (Variables|/Script/Engine.SceneComponent|GetRelativeScale3D (Variables|Default|GetCube))))

(fn ConstructionScript)

(fn AddedScore
  (params (Count :type Integer))
  (bind _output_get (Variables|Default|SetScore (+ (Math|Integer|Absolute(Integer) Count) (Variables|Default|GetScore))))
  (Default|CallScoreChanged _output_get))