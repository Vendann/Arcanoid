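; BP_Ball is the Arcanoid ball, which moves itself on the XY plane and bounces off whatever blocks it.
; Each Tick it sweeps the Sphere along Direction by Speed, then reflects Direction off the hit normal through GetReflectionVector instead of using physics simulation.
; Outside the main menu level, each bounce plays a hit sound and raises Speed up to a cap.
; The DestroyingSmaller event destroys the actor after a delay.
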(event Custom|DestroyingSmaller
  (Utilities|FlowControl|Delay 5.0)
  (Actor|DestroyActor))

(event EventTick
  (params (DeltaSeconds :type Float%20%28single-precision%29))
  (bind _sweephitresult (Transformation|AddWorldOffset (Variables|Default|GetSphere) (* DeltaSeconds (Math|Vector|MakeVector (.x (Variables|Default|GetDirection)) (.y (Variables|Default|GetDirection)) 0.0) (Variables|Default|GetSpeed)) true false))
  (if (.bblockinghit _sweephitresult)
    (Variables|Default|SetDirection (Math|Vector|MakeVector (.x (Math|Vector|GetReflectionVector (Math|Vector|MakeVector (.x (Variables|Default|GetDirection)) (.y (Variables|Default|GetDirection)) 0.0) (.normal _sweephitresult))) (.y (Math|Vector|GetReflectionVector (Math|Vector|MakeVector (.x (Variables|Default|GetDirection)) (.y (Variables|Default|GetDirection)) 0.0) (.normal _sweephitresult))) 0.0))
    (bind _returnvalue (Game|GetCurrentLevelName true))
    (if (Utilities|Enum|NotEqual(Enum) _returnvalue "L_MainMenu")
      (Audio|PlaySoundatLocation "/Game/Arcanoid/Sounds/Hit_Cue.Hit_Cue" (Transformation|GetActorLocation) "0, 0, 0" 1.0 1.0 0.0 0 0 0 0)
      (Variables|Default|SetSpeed (Math|Float|Min(Float) (+ (Variables|Default|GetSpeed) (Variables|Default|GetSpeedIncreaser)) 2e+03)))))

(fn ConstructionScript)