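; BP_Bonus is a bonus pickup actor for the Arcanoid game that randomly becomes a SCALER, HP or BALL type.
; The construction script rolls the type, writes its name to a text render and color-codes both the sphere material and text to match.
; Tick moves the actor along the X component of Direction at Speed with a swept offset.
; The graphs shown apply no bonus effect.
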(event EventTick
  (params (DeltaSeconds :type Float%20%28single-precision%29))
  (Transformation|AddActorWorldOffset (Math|Vector|MakeVector (.x (* DeltaSeconds (Math|Vector|MakeVector (.x (Variables|Default|GetDirection)) 0.0 0.0) (Variables|Default|GetSpeed))) 0.0 0.0) true))

(fn ConstructionScript
  (bind _sphere (Variables|Default|GetSphere))
  (bind _textrender (Variables|Default|GetTextRender))
  (Variables|Default|SetBonusType (Utilities|Select :Index (Math|Random|RandomIntegerinRange 0 2) :Option%200 "NewEnumerator0" :Option%201 "NewEnumerator1" :Option%202 "NewEnumerator2"))
  (Rendering|Components|TextRender|SetText (Variables|Default|GetTextRender) (Utilities|Text|ToText(String) (Utilities|String|EnumtoString (Variables|Default|GetBonusType))))
  (switch Utilities|FlowControl|Switch|SwitchonE_BonusType (Variables|Default|GetBonusType)
    (:NewEnumerator0
      (Rendering|Material|SetMaterial _sphere 0 "/Game/Arcanoid/Materials/MI_Green.MI_Green")
      (Rendering|Components|TextRender|SetTextRenderColor _textrender (Math|Color|MakeColor 0 255 0 0)))
    (:NewEnumerator1
      (Rendering|Material|SetMaterial _sphere 0 "/Game/Arcanoid/Materials/MI_Red.MI_Red")
      (Rendering|Components|TextRender|SetTextRenderColor _textrender (Math|Color|MakeColor 0 0 255 0)))
    (:NewEnumerator2
      (Rendering|Material|SetMaterial _sphere 0 "/Game/Arcanoid/Materials/MI_Blue.MI_Blue")
      (Rendering|Components|TextRender|SetTextRenderColor _textrender (Math|Color|MakeColor 255 0 0 0)))))