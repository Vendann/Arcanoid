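; BP_Cube is a breakable block for the Arcanoid game that loses HP on each BP_Ball hit.
; The construction script randomly makes it a tougher, higher-scoring green cube or a weaker blue one.
; Hits update the material to match remaining HP, and at zero the cube calls CubeDead with its score and destroys itself.
; Green cubes, plus a random share of blue ones, spawn a BP_Bonus when destroyed.
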(event Custom|SpawnBonus
  (params (DestroyedActor :type Actor%20Object%20Reference))
  ;[1 1 1] Begin Play / Bonus Spawner
  (Game|SpawnActorfromClass "/Game/Arcanoid/Blueprints/Bonuses/BP_Bonus.BP_Bonus_C" (Math|Transform|MakeTransform (Transformation|GetActorLocation)) "AlwaysSpawn" "MultiplyWithRoot" 0 0))

(event EventBeginPlay
  ;[1 1 1] Begin Play / Bonus Spawner
  (if (== (Rendering|Material|GetMaterial (Variables|Default|GetCube) 0) "/Game/Arcanoid/Materials/MI_Green.MI_Green")
    (Game|BindEventtoOnDestroyed (delegate Custom|SpawnBonus) :!label _label)
    (elif (>= (Math|Random|RandomFloat) 0.8)
      (goto _label))))

(event Collision|EventHit
  (params (MyComp :type Primitive%20Component%20Object%20Reference) (Other :type Actor%20Object%20Reference) (OtherComp :type Primitive%20Component%20Object%20Reference) (bSelfMoved :type Boolean) (HitLocation :type Vector :default "0, 0, 0") (HitNormal :type Vector :default "0, 0, 0") (NormalImpulse :type Vector :default "0, 0, 0") (Hit :type Hit%20Result%20Structure%20%28by%20ref%29))
  (bind _cube (Variables|Default|GetCube))
  ;[1 1 1] Hit
  (Utilities|Casting|CastToBP_Ball Other)
  (bind _result (Math|Integer|DecrementInt (Variables|Default|GetHP))
    (:%20%20
      (switch int _result
        (:0
          (Default|CallCubeDead (Variables|Default|GetScore))
          (Actor|DestroyActor))
        (:1
          (Rendering|Material|SetMaterial _cube 0 "/Game/Arcanoid/Materials/MI_Blue.MI_Blue"))
        (:2
          (Rendering|Material|SetMaterial _cube 0 "/Game/Arcanoid/Materials/MI_Green.MI_Green"))))))

(fn ConstructionScript
  (bind _cube (Variables|Default|GetCube))
  (if (>= (Math|Random|RandomFloat) 0.7)
    (Rendering|Material|SetMaterial _cube 0 "/Game/Arcanoid/Materials/MI_Green.MI_Green")
    (Variables|Default|SetHP 2)
    (Variables|Default|SetScore 25)
    (else
      (Rendering|Material|SetMaterial _cube 0 "/Game/Arcanoid/Materials/MI_Blue.MI_Blue")
      (Variables|Default|SetHP 1)
      (Variables|Default|SetScore 10))))