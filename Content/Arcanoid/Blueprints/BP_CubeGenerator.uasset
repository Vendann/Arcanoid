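; Arcanoid level generator that spawns an X by Y grid of BP_Cube bricks, spaced by Padding, from the actor's location.
; The construction script builds static mesh previews of the grid, which BeginPlay destroys before spawning the real cubes.
; It binds each cube's death event to add score to the BP_PlayerPawn and fires CubesDestroyed once every cube is dead.
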(event Custom|CubeDead
  (params (Score :type Integer))
  (Default|AddedScore (Variables|Default|GetPlayerPawn) Score)
  (Math|Integer|IncrementInt (Variables|Default|GetDeadCubes)
    (:%20%20
      (if (>= (Variables|Default|GetDeadCubes) (Variables|Default|GetCubesToWin))
        (Default|CallCubesDestroyed)))))

(event EventBeginPlay
  (bind _returnvalue (Transformation|GetActorLocation))
  (Utilities|FlowControl|Sequence
    (:then_0
      (bind _returnvalue_2 (Actor|GetActorOfClass "/Game/Arcanoid/Blueprints/Core/BP_PlayerPawn.BP_PlayerPawn_C"))
      (Variables|Default|SetPlayerPawn _returnvalue_2))
    (:then_1
      (for _array_element (Variables|Default|GetPreviewArray)
        (Components|DestroyComponent _array_element))
      (for _index (range 0 (- (Variables|Default|GetX) 1))
        (for _index_2 (range 0 (- (Variables|Default|GetY) 1))
          (bind _returnvalue_3 (Game|SpawnActorfromClass "/Game/Arcanoid/Blueprints/BP_Cube.BP_Cube_C" (Math|Transform|MakeTransform (Math|Vector|MakeVector (+ (Math|Conversions|ToFloat(Integer) (* _index (Variables|Default|GetPadding))) (.x _returnvalue)) (+ (Math|Conversions|ToFloat(Integer) (* _index_2 (Variables|Default|GetPadding))) (.y _returnvalue)) (.z _returnvalue))) "Undefined" "MultiplyWithRoot" 0 0))
          (Utilities|Array|Add (Variables|Default|GetCubesArray) _returnvalue_3)))
      (bind _cubescount (CallFunction|CubesCount))
      (Variables|Default|SetCubesToWin _cubescount)
      (for _array_element_2 (Variables|Default|GetCubesArray)
        (EventDispatchers|BindEventtoCubeDead _array_element_2 (delegate Custom|CubeDead))))))

(fn ConstructionScript
  (for _index (range 0 (- (Variables|Default|GetX) 1))
    (for _index_2 (range 0 (- (Variables|Default|GetY) 1))
      (bind _returnvalue (AddComponent|AddStaticMeshComponent false (Math|Transform|MakeTransform (Math|Vector|MakeVector (Math|Conversions|ToFloat(Integer) (* _index (Variables|Default|GetPadding))) (Math|Conversions|ToFloat(Integer) (* _index_2 (Variables|Default|GetPadding))) 0.0))))
      (Utilities|Array|Add (Variables|Default|GetPreviewArray) _returnvalue))))

(fn CubesCount
  (return (Utilities|Array|Length (Variables|Default|GetCubesArray))))